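; Sprint component that doubles the player's walk speed and manages an endurance gauge.
; Looping timers drain endurance during sprint and refill it once sprinting stops.
; An empty gauge sets a tired state that blocks sprinting until fully refilled, and falling also ends the sprint.
; Dispatcher calls broadcast level updates and depletion, replenishment or tired states to listeners.
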(event `StopEnduranceDepletion`
  ;[1 1 1] Epuisement du niveau d'endurance
  (if (`KismetSystemLibrary.K2_IsTimerActiveHandle` (stale `StartEnduranceDepletion` _returnvalue))
    (`KismetSystemLibrary.K2_ClearAndInvalidateTimerHandle` (stale `StartEnduranceDepletion` _returnvalue))))

(event `StartEnduranceDepletion`
  ;[1 1 1] Epuisement du niveau d'endurance
  (`self.SetDepletionState`)
  (bind _returnvalue (`KismetSystemLibrary.K2_SetTimerDelegate` (delegate `DepleteEndurance`) (* (`self.DepletionDuration`) (`self.DepletionRate`)) true)))

(event `self.ReceiveBeginPlay`
  (set `self.DefaultWalkSpeed` (`CharacterMovementComponent.MaxWalkSpeed` (`self.PlayerMovementComponent`)))
  (set `self.SprintSpeed` (* (`self.DefaultWalkSpeed`) 2.0))
  (set `self.CurrentEnduranceLevel` (`self.MaxEnduranceLevel`)))

(event `DepleteEndurance`
  ;[1 1 1] Epuisement du niveau d'endurance
  (set `self.CurrentEnduranceLevel` (- (`self.CurrentEnduranceLevel`) (`self.DepletionRate`)))
  (`self.UpdateEnduranceLevel`)
  (if (<= (`self.CurrentEnduranceLevel`) 0.0)
    (set `self.bIsTired` true)
    (set `self.CurrentEnduranceLevel` 0.0)
    (`self.StopSprint`)
    (elif (`NavMovementComponent.IsFalling` (`self.PlayerMovementComponent`))
      (`self.StopSprint`))))

(event `StartSprint`
  (if (and (not (`self.bIsSprinting`)) (not (`self.bIsTired`)))
    (set `self.bIsSprinting` true)
    (set `CharacterMovementComponent.MaxWalkSpeed` (`self.SprintSpeed`) (`self.PlayerMovementComponent`))
    (`self.StartEnduranceDepletion`)))

(event `StopSprint`
  (if (`self.bIsSprinting`)
    (set `self.bIsSprinting` false)
    (set `CharacterMovementComponent.MaxWalkSpeed` (`self.DefaultWalkSpeed`) (`self.PlayerMovementComponent`))
    (`self.StopEnduranceDepletion`)
    (`self.StartEnduranceReplenishment`)))

(event `StopEnduranceReplenishment`
  ;[1 1 1] Remplissage du niveau d'endurance
  (if (`KismetSystemLibrary.K2_IsTimerActiveHandle` (stale `StartEnduranceReplenishment` _returnvalue))
    (`KismetSystemLibrary.K2_ClearAndInvalidateTimerHandle` (stale `StartEnduranceReplenishment` _returnvalue))))

(event `StartEnduranceReplenishment`
  ;[1 1 1] Remplissage du niveau d'endurance
  (if (`self.bIsTired`)
    (`self.SetTiredState`)
    (else
      (`self.SetReplenishmentState`)))
  (bind _returnvalue (`KismetSystemLibrary.K2_SetTimerDelegate` (`|CreateDelegate` :!event `ReplenishEndurance`) (* (`self.ReplenishDuration`) (`self.EnduranceRate`)) true)))

(event `ReplenishEndurance`
  ;[1 1 1] Remplissage du niveau d'endurance
  (set `self.CurrentEnduranceLevel` (+ (`self.CurrentEnduranceLevel`) (`self.EnduranceRate`)))
  (`self.UpdateEnduranceLevel`)
  (if (>= (`self.CurrentEnduranceLevel`) (`self.MaxEnduranceLevel`))
    (set `self.bIsTired` false)
    (set `self.CurrentEnduranceLevel` (`self.MaxEnduranceLevel`))
    (`self.StopEnduranceReplenishment`)
    (`self.SetReplenishmentState`)))