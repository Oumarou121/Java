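; BP_CryonisBlock is the block actor of the Cryonis module, which grows up from the ground when spawned.
; On BeginPlay it flattens its root to zero Z scale, then GrowTimeline drives that Z scale from its Factor track.
; The timeline play rate is the inverse of GrowDuration, so that variable sets the growth time.
; TriggerDestroy removes the block immediately by destroying the actor.
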(event `self.ReceiveBeginPlay`
  (bind _defaultsceneroot (`self.DefaultSceneRoot`))
  (bind (_returnvalue_x _returnvalue_y) (`KismetMathLibrary.BreakVector` (`SceneComponent.K2_GetComponentScale` _defaultsceneroot)))
  (`TimelineComponent.SetPlayRate` (`self.GrowTimeline`) (/ 1.0 (`self.GrowDuration`)))
  ;[1 1 1] Faire grandir le block au sol
  (`SceneComponent.SetWorldScale3D` (`self.DefaultSceneRoot`) (1.0 1.0 0.0))
  (bind (_direction _factor) (`Timeline|GrowTimeline`)
    (:`Update`
      (`SceneComponent.SetWorldScale3D` _defaultsceneroot (`KismetMathLibrary.MakeVector` _returnvalue_x _returnvalue_y _factor)))))

(event `TriggerDestroy`
  (`self.K2_DestroyActor`))

(fn `UserConstructionScript`)