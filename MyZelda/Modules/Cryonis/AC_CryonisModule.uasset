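; Actor component for a Cryonis-style ability that lets the player create ice blocks on surfaces tagged Cryonisable, or destroy existing ones.
; While active, a looping timer line-traces from the follow camera, caching either a valid surface point and normal or a targeted BP_CryonisBlock.
; A Niagara preview follows valid hits, aligned to the normal.
; SpawnBlock plays a cast montage and spawns a block there, or triggers the targeted block's destruction.
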(event `SpawnPS`
  ;[0 0 0 1 24] Gére le system de particule
  (bind _returnvalue (`NiagaraFunctionLibrary.SpawnSystemAtLocation` "/Game/MyZelda/Modules/Cryonis/NiagaraPS/NE_CryonisBlock_System.NE_CryonisBlock_System"))
  (set `self.PS` _returnvalue))

(event `DestroyPS`
  ;[0 0 0 1 24] Gére le system de particule
  (`self.K2_DestroyComponent` (`self.PS`)))

(event `HidePS`
  ;[0 0 0 1 24] Gére le system de particule
  (`SceneComponent.SetVisibility` (`self.PS`) false false))

(event `ShowPS`
  (bind _ps (`self.PS`))
  ;[0 0 0 1 24] Gére le system de particule
  (`SceneComponent.SetVisibility` _ps true false)
  (`SceneComponent.K2_SetWorldLocationAndRotation` _ps (`self.ValideZoneHitLoaction`) (`KismetMathLibrary.MakeRotFromZ` (`self.ValideZoneNormal`)) false false))

(event `ClearSearchVariables`
  ;[0 0 0 1 24] Réinitialise tout ce aui est relatif à la recherche de surface valide
  (set `self.bHasHitValideZone` false)
  (set `self.bHasHitBlock` false)
  (set `self.ValideZoneHitLoaction` (0.0 0.0 0.0))
  (set `self.ValideZoneNormal` (0.0 0.0 0.0))
  (set `self.TargetHitBlock` null))

(event `TriggerSpawningAnim`
  ;[0 0 0 1 24] Lance l'animation du joueur aui fait apparaitre un block
  (`|PlayMontage` (`Character.Mesh` (`self.Player`)) "/Game/MyZelda/Animations/Cast_Montage.Cast_Montage"
    (:`then`
      (set `self.bIsSpawingBlock` true)
      (`self.HidePS`))
    (:`OnCompleted`
      (set `self.bIsSpawingBlock` false)
      (`self.ShowPS`))))

(event `SpawnBlock`
  ;[0 0 0 1 24] Fait apparaitre un block ou effache le un block
  (if (and (`self.bIModuleActived`) (or (`self.bHasHitBlock`) (`self.bHasHitValideZone`)))
    (if (`self.bHasHitValideZone`)
      (`self.TriggerSpawningAnim`)
      (`|SpawnActorFromClass` "/Game/MyZelda/Modules/Cryonis/BP_CryonisBlock.BP_CryonisBlock_C" (`KismetMathLibrary.MakeTransform` (`self.ValideZoneHitLoaction`) (`KismetMathLibrary.MakeRotFromZ` (`self.ValideZoneNormal`))) "Undefined" "OverrideRootScale" null null)
      (`self.ClearSearchVariables`)
      (else
        (`/Game/MyZelda/Modules/Cryonis/BP_CryonisBlock.TriggerDestroy` (`self.TargetHitBlock`))
        (`self.ClearSearchVariables`)))))

(event `ActivatedModule`
  ;[0 0 0 1 24] Lance de recherche de block ou de zone
  (if (and (not (`self.bIModuleActived`)) (not (`self.bIsSpawingBlock`)))
    (`KismetSystemLibrary.PrintString` "ACTIVATION CRYONIS")
    (set `self.bIModuleActived` true)
    (`self.SpawnPS`)
    (`self.StartSearching`)
    (else
      (`self.StopSearching`)
      (`self.ClearSearchVariables`)
      (`KismetSystemLibrary.PrintString` "CRYONIS INACTIVE")
      (set `self.bIModuleActived` false)
      (`self.DestroyPS`))))

(event `StopSearching`
  ;[0 0 0 1 24] Lance un rayon dans le monde pour cherche une zone valide ou un block
  (`KismetSystemLibrary.K2_ClearAndInvalidateTimerHandle` (stale `StartSearching` _returnvalue)))

(event `StartSearching`
  ;[0 0 0 1 24] Lance un rayon dans le monde pour cherche une zone valide ou un block
  (bind _returnvalue (`KismetSystemLibrary.K2_SetTimerDelegate` (delegate `Search`) 0.1 true)))

(event `Search`
  (bind _followcamera (`/Game/MyZelda/Blueprints/BP_Zelda.FollowCamera` (`self.Player`)))
  (bind _returnvalue (`SceneComponent.K2_GetComponentLocation` _followcamera))
  ;[0 0 0 1 24] Lance un rayon dans le monde pour cherche une zone valide ou un block
  (if (not (`self.bIsSpawingBlock`))
    ;;[1 1 1] Lance un rayon depuis le reticule jusque dans le monde
    (bind (_outhit _returnvalue_2) (`KismetSystemLibrary.LineTraceSingle` _returnvalue (+ _returnvalue (* (`SceneComponent.GetForwardVector` _followcamera) (`self.Range`))) "TraceTypeQuery1"))
    (if _returnvalue_2
      (bind (_bblockinghit _binitialoverlap _time _distance _location _impactpoint _normal _impactnormal _physmat _hitactor) (`GameplayStatics.BreakHitResult` _outhit))
      ;;[1 1 1] Si on touche une zone cryonisable on stocke les données
      (if (`Actor.ActorHasTag` _hitactor "Cryonisable")
        (set `self.bHasHitValideZone` true)
        (set `self.ValideZoneHitLoaction` _location)
        (set `self.ValideZoneNormal` _normal)
        (`self.ShowPS`)
        (else
          (set `self.bHasHitValideZone` false)
          ;;[1 1 1] Si on à toucher un block on stock le block en question
          (bind _asbp_cryonis_block (cast `/Game/MyZelda/Modules/Cryonis/BP_CryonisBlock` _hitactor)
            (:`then`
              (set `self.TargetHitBlock` _asbp_cryonis_block)
              (set `self.bHasHitBlock` true)
              (`self.HidePS`))
            (:`CastFailed`
              (set `self.bHasHitBlock` false)
              (`self.ClearSearchVariables`)
              (`self.HidePS`)))))
      (else
        (`self.ClearSearchVariables`)
        (`self.HidePS`)))))