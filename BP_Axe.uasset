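; Throwable axe actor that flies spinning toward a target, sticks into what it hits and can be recalled to the player, like a boomerang.
; Throw drives projectile and rotating movement; on hit, a sphere trace aligns the axe to the surface.
; Callback switches collision profile and uses a timeline along a quadratic Bézier arcing to the hand socket, then calls GrabAxe.
; Overlaps deal point damage; ribbon trail, impact particles and a charging material parameter provide feedback.
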(event `Callback`
  (params (Player :type "/Game/GodOfWar/BP_Player Object Reference"))
  (if (`self.bThrow`)
    (set `self.bThrow` false)
    (`self.ActivateTrail`)
    (`PrimitiveComponent.SetCollisionProfileName` (`self.StaticMesh`) "AxeCalled" true)
    (`ActorComponent.Deactivate` (`self.ProjectileMovement`))
    (set `RotatingMovementComponent.RotationRate` (`self.CallbackRotationRate`) (`self.RotatingMovement`))
    (`ActorComponent.Activate` (`self.RotatingMovement`) true)
    (`self.K2_SetActorRotation` (`KismetMathLibrary.FindLookAtRotation` (`self.K2_GetActorLocation`) (`self.K2_GetActorLocation` Player)))
    (set `self.CallbackInitialLoc` (`self.K2_GetActorLocation`))
    (set `self.CallbackIntermediateLoc` (+ (`self.K2_GetActorLocation` Player) (* (`self.GetActorForwardVector` Player) 500.0) (* (`self.GetActorRightVector` Player) 500.0)))
    (bind (_direction _factor) (`Timeline|CallbackTimeline` :!via `PlayFromStart`)
      (:`Update`
        (`self.K2_SetActorLocation` (`self.ComputeQuadratic` (`self.CallbackInitialLoc`) (`self.CallbackIntermediateLoc`) (`SceneComponent.GetSocketLocation` (`Character.Mesh` Player) "WeaponSocket2") _factor) true))
      (:`Finished`
        (`ActorComponent.Deactivate` (`self.RotatingMovement`))
        (`/Game/GodOfWar/BP_Player.GrabAxe` Player)
        (`ActorComponent.Activate` (`self.ImpactPS`) true)
        (`self.DeactivateTrail`)))))

(event `Stop`
  (`ActorComponent.Deactivate` (`self.ProjectileMovement`))
  (`ActorComponent.Deactivate` (`self.RotatingMovement`))
  (`self.DeactivateTrail`))

(event `self.StaticMesh.OnComponentHit`
  (params (HitComponent :type "PrimitiveComponent Object Reference") (OtherActor :type "Actor Object Reference") (OtherComp :type "PrimitiveComponent Object Reference") (NormalImpulse :type "Vector Structure") (Hit :type "HitResult Structure (by ref)"))
  (bind _returnvalue (`self.K2_GetActorLocation`))
  (if (`self.bThrow`)
    (`self.Stop`)
    (`self.K2_SetActorRotation` (`KismetMathLibrary.MakeRotFromX` (`KismetMathLibrary.NegateVector` (`.ImpactNormal` (`GameplayStatics.BreakHitResult` Hit)))))
    (bind (_outhit _returnvalue_2) (`KismetSystemLibrary.SphereTraceSingle` _returnvalue (+ _returnvalue (* (`self.ThrowDirection`) 200.0)) 50.0 "TraceTypeQuery1"))
    (if _returnvalue_2
      (`self.K2_SetActorLocation` (+ (`.ImpactPoint` (`GameplayStatics.BreakHitResult` _outhit)) (- (`SceneComponent.K2_GetComponentLocation` (`self.StaticMesh`)) (`SceneComponent.K2_GetComponentLocation` (`self.Arrow`)))) false true))))

(event `self.ReceiveBeginPlay`
  (`TimelineComponent.SetPlayRate` (`self.CallbackTimeline`) (/ 1.0 0.7)))

(event `self.StaticMesh.OnComponentBeginOverlap`
  (params (OverlappedComponent :type "PrimitiveComponent Object Reference") (OtherActor :type "Actor Object Reference") (OtherComp :type "PrimitiveComponent Object Reference") (OtherBodyIndex :type Integer) (bFromSweep :type Boolean) (SweepResult :type "HitResult Structure (by ref)"))
  (`GameplayStatics.ApplyPointDamage` (`.HitActor` (`GameplayStatics.BreakHitResult` SweepResult)) 10.0 (`self.K2_GetActorLocation`) (`GameplayStatics.MakeHitResult` false false 0.0 0.0 (0.0 0.0 0.0) (0.0 0.0 0.0) (0.0 0.0 1.0) (0.0 0.0 1.0) "/Game/FunkyShooterAAA/Core/Enemy/PM_Body.PM_Body") (`GameplayStatics.GetPlayerController` 0) (`GameplayStatics.GetPlayerCharacter` 0)))

(fn `ActivateTrail`
  (`ActorComponent.Activate` (`self.RibbonPS`) true))

(fn `ComputeQuadratic`
  (params (P0 :type "Vector Structure") (P1 :type "Vector Structure") (P2 :type "Vector Structure") (T :type "Float (double-precision)"))
  (returns (ReturnValue :type "Vector Structure"))
  (bind _returnvalue (- 1.0 T))
  (return (+ (* P0 (`KismetMathLibrary.MultiplyMultiply_FloatFloat` _returnvalue 2.0)) (* P1 (* _returnvalue 2.0 T)) (* P2 (`KismetMathLibrary.MultiplyMultiply_FloatFloat` T 2.0)))))

(fn `DeactivateTrail`
  (`ActorComponent.Deactivate` (`self.RibbonPS`)))

(fn `SetChargingState`
  (params (bIsCharging :type Boolean))
  (bind _returnvalue (`PrimitiveComponent.CreateDynamicMaterialInstance` (`self.StaticMesh`) 0 "/Game/GodOfWar/Axe/M_Axe.M_Axe" "None"))
  (`MaterialInstanceDynamic.SetScalarParameterValue` _returnvalue "Charging" (`KismetMathLibrary.SelectFloat` 1.0 0.0 bIsCharging)))

(fn `Throw`
  (params (Destination :type "Vector Structure"))
  (bind _projectilemovement (`self.ProjectileMovement`))
  (bind _rotatingmovement (`self.RotatingMovement`))
  (`|ExecutionSequence`
    (:`then_0`
      (set `self.ThrowDirection` (`KismetMathLibrary.Normal` (- Destination (`self.K2_GetActorLocation`))))
      (set `self.bThrow` true)
      (`ActorComponent.Activate` _projectilemovement true)
      (set `MovementComponent.Velocity` (* (`self.ThrowDirection`) (`self.Speed`)) _projectilemovement))
    (:`then_1`
      (set `RotatingMovementComponent.RotationRate` (`self.ThrowRotationRate`) _rotatingmovement)
      (`ActorComponent.Activate` _rotatingmovement true)
      (`PrimitiveComponent.SetCollisionProfileName` (`self.StaticMesh`) "AxeThrown" true)
      (`self.ActivateTrail`))))

(fn `UserConstructionScript`)