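; AC_EnergyGun is the energy gun logic for the player, with separate charge and fire events.
; ChargeGun spawns a BP_Projectile_EG at the player mesh's Muzzle_01 socket, attaches it there and stores it.
; FireGun line-traces from screen center out to Range, rotates the stored projectile toward the hit point or trace end, then launches it, so shots converge on the crosshair despite the muzzle offset.
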(event `ChargeGun`
  (bind _mesh (`Character.Mesh` (`GameplayStatics.GetPlayerCharacter` 0)))
  (bind _returnvalue_location (`KismetMathLibrary.BreakTransform` (`SceneComponent.GetSocketTransform` _mesh "Muzzle_01" "RTS_World")))
  (bind _returnvalue (`|SpawnActorFromClass` "/Game/FunkyShooterAAA/Core/EnergyGun/BP_Projectile_EG.BP_Projectile_EG_C" (`KismetMathLibrary.MakeTransform` _returnvalue_location) "Undefined" "OverrideRootScale" null null))
  (bind _output_get (set `self.Projectile` _returnvalue))
  (`Actor.K2_AttachToComponent` _output_get _mesh "Muzzle_01" "KeepWorld" "SnapToTarget" "SnapToTarget" true))

(event `FireGun`
  (bind (_worldposition _worlddirection) (`GameplayStatics.DeprojectScreenToWorld` (`GameplayStatics.GetPlayerController` 0) (* (`WidgetLayoutLibrary.GetViewportSize`) 0.5)))
  (bind _outhit (`KismetSystemLibrary.LineTraceSingle` _worldposition (+ _worldposition (* _worlddirection (`self.Range`))) "TraceTypeQuery3"))
  (bind _projectile (`self.Projectile`)
    (:`then`
      (bind (_bblockinghit _binitialoverlap _time _distance _location _impactpoint _normal _impactnormal _physmat _hitactor _hitcomponent _hitbonename _hititem _elementindex _faceindex _tracestart _traceend) (`GameplayStatics.BreakHitResult` _outhit))
      (`Actor.K2_SetActorRotation` _projectile (`KismetMathLibrary.FindLookAtRotation` (`Actor.K2_GetActorLocation` _projectile) (`KismetMathLibrary.SelectVector` _location _traceend _bblockinghit)) false)
      (`/Game/FunkyShooterAAA/Core/EnergyGun/BP_Projectile_EG.Launch` _projectile))
    (:`else`)))