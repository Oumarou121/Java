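; Chargeable energy gun projectile that grows while held and deals point damage scaled by its size on impact.
; On spawn, a timeline scales the actor from 1x to 3x, stopping the charge effect when finished.
; Launch freezes growth, detaches the projectile, attaches a size-matched Niagara trail, fires it along local forward and destroys it after its lifetime.
; Collision hits spawn an impact effect and destroy the actor.
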(event `self.ReceiveBeginPlay`
  (bind (_direction _lerp) (`Timeline|Tgrow_Templete` :!label _label)
    (:`Update`
      (`self.SetActorScale3D` (`KismetMathLibrary.VLerp` (1.0 1.0 1.0) (3.0 3.0 3.0) _lerp)))
    (:`Finished`
      (`ActorComponent.Deactivate` (`self.NE_Charge_System`)))))

(event `Launch`
  (bind _returnvalue_x (`KismetMathLibrary.BreakVector` (`self.GetActorScale3D`)))
  (bind _returnvalue_x_2 (`KismetMathLibrary.BreakVector` (`SceneComponent.K2_GetComponentScale` (`self.Sphere`))))
  (`ActorComponent.Deactivate` (`self.NE_Charge_System`))
  (`|ExecutionSequence`
    (:`then_0`
      (goto _label :!via `Stop`))
    (:`then_1`
      (`self.K2_DetachFromActor` "KeepWorld" "KeepWorld" "KeepWorld")
      (bind _returnvalue (`NiagaraFunctionLibrary.SpawnSystemAttached` "/Game/FunkyShooterAAA/Core/EnergyGun/NE_Trail_System.NE_Trail_System" (`self.Collision`) "None" (0.0 0.0 0.0) (struct) "SnapToTarget" true))
      (`FXSystemComponent.SetFloatParameter` _returnvalue "Size" (* _returnvalue_x _returnvalue_x_2))
      (`ProjectileMovementComponent.SetVelocityInLocalSpace` (`self.ProjectileMovement`) (2000.0 0.0 0.0))
      (`KismetSystemLibrary.Delay` (`self.Lifetime`))
      (`self.K2_DestroyActor`))))

(event `self.Collision.OnComponentHit`
  (params (HitComponent :type "PrimitiveComponent Object Reference") (OtherActor :type "Actor Object Reference") (OtherComp :type "PrimitiveComponent Object Reference") (NormalImpulse :type "Vector Structure") (Hit :type "HitResult Structure (by ref)"))
  (bind _returnvalue_x (`KismetMathLibrary.BreakVector` (`self.GetActorScale3D`)))
  (`GameplayStatics.ApplyPointDamage` OtherActor (* (`self.Base Damage`) _returnvalue_x) (`self.K2_GetActorLocation`) (`GameplayStatics.MakeHitResult` false false 0.0 0.0 (0.0 0.0 0.0) (0.0 0.0 0.0) (0.0 0.0 1.0) (0.0 0.0 1.0) "/Game/FunkyShooterAAA/Core/Enemy/PM_Body.PM_Body"))
  (`NiagaraFunctionLibrary.SpawnSystemAtLocation` "/Game/FunkyShooterAAA/Core/EnergyGun/NE_Hit_System.NE_Hit_System" (`self.K2_GetActorLocation`))
  (`self.K2_DestroyActor`))

(fn `UserConstructionScript`)