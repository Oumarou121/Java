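; Aim-assist component that computes a corrected crosshair screen position on a 60 Hz looping timer, with an optional debug HUD.
; A sphere trace from screen center selects the pawn hit closest to center.
; Concentric screen-space zones snap the crosshair to BPI_Damageable weak or base spots, or other pawns' hit points, or bend it proportionally toward the target.
; Getters expose the crosshair position and a magnetism factor for the magnetic zone.
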(event `self.ReceiveBeginPlay`
  (bind _returnvalue (`GameplayStatics.GetPlayerController` 0))
  (`|ExecutionSequence`
    (:`then_0`
      (if (`self.bIsDebugActivated`)
        (`PlayerController.ClientSetHUD` _returnvalue "/Game/FunkyShooterAAA/Core/AimingSytem/BPH_AimingSystem_Debug.BPH_AimingSystem_Debug_C")
        (set `self.Debug HUD` (cast `/Game/FunkyShooterAAA/Core/AimingSytem/BPH_AimingSystem_Debug` (`PlayerController.GetHUD` _returnvalue) :!pure true))
        (set `/Game/FunkyShooterAAA/Core/AimingSytem/BPH_AimingSystem_Debug.HeadshotZoneRaduis` (`self.Headshot Zone Raduis`) (`self.Debug HUD`))
        (set `/Game/FunkyShooterAAA/Core/AimingSytem/BPH_AimingSystem_Debug.BaseshotZoneRaduis` (`self.Baseshot Zone Raduis`) (`self.Debug HUD`))
        (set `/Game/FunkyShooterAAA/Core/AimingSytem/BPH_AimingSystem_Debug.BendshotZoneRaduis` (`self.Bend Zone Raduis`) (`self.Debug HUD`))
        (set `/Game/FunkyShooterAAA/Core/AimingSytem/BPH_AimingSystem_Debug.MagneticshotZoneRaduis` (`self.Magneticshot Zone Raduis`) (`self.Debug HUD`))
        (`/Game/FunkyShooterAAA/Core/AimingSytem/BPH_AimingSystem_Debug.Initialize` (`self.Debug HUD`))))
    (:`then_1`
      (`KismetSystemLibrary.K2_SetTimerDelegate` (delegate `ExecuteSystem`) 0.016667 true))))

(event `ExecuteSystem`
  (bind _debug_hud (`self.Debug HUD`))
  (bind (_bwaspawnfound _pawnsreenlocation _bdoesimplementinterface _basespotscreenlocation _weakspotscreenlocation) (`self.SearchForPawnToEngageOn`))
  (bind _adjustedcrosshair (`self.AdjustCrosshairScreenLocation` _bwaspawnfound _pawnsreenlocation _bdoesimplementinterface _basespotscreenlocation _weakspotscreenlocation))
  (set `self.CrosshairScreenLocation` _adjustedcrosshair)
  (if (`self.bIsDebugActivated`)
    (set `/Game/FunkyShooterAAA/Core/AimingSytem/BPH_AimingSystem_Debug.MainCrosshairLocation` (`self.CrosshairScreenLocation`) _debug_hud)
    (set `/Game/FunkyShooterAAA/Core/AimingSytem/BPH_AimingSystem_Debug.CurrentSystemState` (`self.CurrentState`) _debug_hud)))

(fn `AdjustCrosshairScreenLocation`
  (params (bWasPawnFound :type Boolean) (EngagedPawnScreenLocation :type "Vector2D Structure") (bDeosImplementInterface :type Boolean) (`Base Spot Screen Location` :type "Vector2D Structure") (`Weak Spot Screen Location` :type "Vector2D Structure"))
  (returns (AdjustedCrosshair :type "Vector2D Structure"))
  (locals (L_EngagedPawnscreenLocation :type "Vector2D Structure") (L_viewportCenterLocation :type "Vector2D Structure") (L_EngagedPawnDistToCenter :type "Float (double-precision)") (LWasPawnFound :type Boolean) (LDeosImplementInterface :type Boolean) (LBaseSpotScreenLocation :type "Vector2D Structure") (LWeakSpotScreenLocation :type "Vector2D Structure"))
  (set `local.LWasPawnFound` bWasPawnFound)
  (set `local.L_EngagedPawnscreenLocation` EngagedPawnScreenLocation)
  (set `local.LDeosImplementInterface` bDeosImplementInterface)
  (set `local.LBaseSpotScreenLocation` `Base Spot Screen Location`)
  (set `local.LWeakSpotScreenLocation` `Weak Spot Screen Location`)
  (set `local.L_viewportCenterLocation` (* (`WidgetLayoutLibrary.GetViewportSize`) 0.5))
  (set `local.L_EngagedPawnDistToCenter` (`KismetMathLibrary.Distance2D` (`local.L_EngagedPawnscreenLocation`) (`local.L_viewportCenterLocation`)))
  (if (and (`local.LWasPawnFound`) (<= (`local.L_EngagedPawnDistToCenter`) (`self.Bend Zone Raduis`)))
    (if (`local.LDeosImplementInterface`)
      (if (<= (`KismetMathLibrary.Distance2D` (`local.LWeakSpotScreenLocation`) (`local.L_viewportCenterLocation`)) (`self.Headshot Zone Raduis`))
        (set `self.CurrentState` "NewEnumerator5")
        (return (`local.LWeakSpotScreenLocation`))
        (elif (<= (`local.L_EngagedPawnDistToCenter`) (`self.Baseshot Zone Raduis`))
          (set `self.CurrentState` "NewEnumerator4")
          (return (`local.LBaseSpotScreenLocation`))
          (else
            _)))
      (elif (<= (`local.L_EngagedPawnDistToCenter`) (`self.Baseshot Zone Raduis`))
        (set `self.CurrentState` "NewEnumerator3")
        (return (`local.L_EngagedPawnscreenLocation`))
        (else
          _)))
    (set `self.CurrentState` "NewEnumerator2")
    (return (+ (`local.L_viewportCenterLocation`) (* (`KismetMathLibrary.Normal2D` (- (`local.L_EngagedPawnscreenLocation`) (`local.L_viewportCenterLocation`))) (/ (* (`self.Baseshot Zone Raduis`) (- (`self.Bend Zone Raduis`) (`local.L_EngagedPawnDistToCenter`))) (- (`self.Bend Zone Raduis`) (`self.Baseshot Zone Raduis`))))))
    (else
      (set `self.CurrentState` (select `bool` (<= (`local.L_EngagedPawnDistToCenter`) (`self.Magneticshot Zone Raduis`)) :`false` "NewEnumerator0" :`true` "NewEnumerator1" :!type "/Game/FunkyShooterAAA/Core/AimingSytem/EAimingState Enum"))
      (return (`local.L_viewportCenterLocation`)))))

(fn `GetCrosshairLocation`
  (returns (CrosshairScreenLocation :type "Vector2D Structure"))
  (return (`self.CrosshairScreenLocation`)))

(fn `GetMagnetismFactor`
  (returns (OutputReselt :type "Float (double-precision)"))
  (return (`KismetMathLibrary.SelectFloat` (`self.MagnetismFactor`) 1.0 (`|EnumEquality` (`self.CurrentState`) "NewEnumerator1"))))

(fn `SearchForPawnToEngageOn`
  (returns (bWasPawnFound :type Boolean) (PawnSreenLocation :type "Vector2D Structure") (bDoesImplementInterface :type Boolean) (BaseSpotScreenLocation :type "Vector2D Structure") (WeakSpotScreenLocation :type "Vector2D Structure"))
  (locals (L_HittedPawns :type "Array of HitResult Structure") (L_HittedPawnDistToCenter :type "Array of Float (double-precision)") (LEngagedPawnScreenLocation :type "Vector2D Structure") (LEngagedPawn :type "Actor Object Reference"))
  (bind _lengagedpawn (`local.LEngagedPawn`))
  (bind (_worldposition _worlddirection) (`GameplayStatics.DeprojectScreenToWorld` (`GameplayStatics.GetPlayerController` 0) (* (`WidgetLayoutLibrary.GetViewportSize`) 0.5)))
  (bind (_bblockinghit _binitialoverlap _time _distance _location _impactpoint _normal _impactnormal _physmat _hitactor) (`GameplayStatics.BreakHitResult` (`|GetArrayItem` (`local.L_HittedPawns`) (`KismetMathLibrary.MinOfFloatArray` (`local.L_HittedPawnDistToCenter`)))))
  (bind (_outhits _returnvalue) (`KismetSystemLibrary.SphereTraceMultiForObjects` (+ _worldposition (* _worlddirection (`self.SearchTraceStartOffset`))) (+ _worldposition (* _worlddirection (`self.SearchTraceRange`))) (`self.SearchTraceSphereRadius`) (`|MakeArray` "ObjectTypeQuery3" :!type "EObjectTypeQuery Enum") false (`|MakeArray` (`GameplayStatics.GetPlayerPawn` 0) :!type "Actor Object Reference") "None" false))
  (set `local.L_HittedPawns` _outhits)
  (if _returnvalue
    (for _index (range (`KismetArrayLibrary.Array_Length` (`local.L_HittedPawns`)))
      (`KismetArrayLibrary.Array_Add` (`local.L_HittedPawnDistToCenter`) (`KismetMathLibrary.Distance2D` (* (`WidgetLayoutLibrary.GetViewportSize`) 0.5) (`GameplayStatics.ProjectWorldToScreen` (`GameplayStatics.GetPlayerController` 0) (`.ImpactPoint` (`GameplayStatics.BreakHitResult` (`|GetArrayItem` (`local.L_HittedPawns`) _index)))))))
    (set `local.LEngagedPawnScreenLocation` (`GameplayStatics.ProjectWorldToScreen` (`GameplayStatics.GetPlayerController` 0) _impactpoint))
    (set `local.LEngagedPawn` _hitactor)
    (if (`KismetSystemLibrary.DoesImplementInterface` (`local.LEngagedPawn`) "/Game/FunkyShooterAAA/Core/Enemy/BPI_Damageable.BPI_Damageable_C")
      (bind _screenlocation (message `/Game/FunkyShooterAAA/Core/Enemy/BPI_Damageable.GetWeakSpotScreenLocation` _lengagedpawn))
      (bind _screenlocation_2 (message `/Game/FunkyShooterAAA/Core/Enemy/BPI_Damageable.GetBaseSpotScrrenLocation` _lengagedpawn))
      (return true (`local.LEngagedPawnScreenLocation`) true _screenlocation_2 _screenlocation)
      (else
        (return true (`local.LEngagedPawnScreenLocation`) false (0.0 0.0) (0.0 0.0))))
    (else
      (return false (-1.0 -1.0) false (0.0 0.0) (0.0 0.0)))))