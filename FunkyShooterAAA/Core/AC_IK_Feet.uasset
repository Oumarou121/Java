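; Foot IK component that computes foot offsets, foot rotations and a pelvis offset to adapt a character to uneven ground.
; Each tick it line-traces down at each foot bone from capsule-center height, measuring the floor's distance below the capsule bottom and its normal.
; The pelvis follows the larger foot offset, while each foot rotates from actor up toward its floor normal.
; All outputs are smoothed with interpolation.
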(event `self.ReceiveTick`
  (params (DeltaSeconds :type "Float (single-precision)"))
  (set `self.Delta Seconds` DeltaSeconds)
  ;[1 1 1] Foot_l
  (bind (_returnvalue _impactnormal) (`self.TraceFromFoot` (`self.LeftFootName`) (`self.Trace Dist Below Capscule`)))
  (set `self.LeftFootFoorNormal` _impactnormal)
  (set `self.LeftFootOffset` (`KismetMathLibrary.FInterpTo` (`self.LeftFootOffset`) _returnvalue (`self.Delta Seconds`) (`self.Interp Speed`)))
  ;[1 1 1] Foot_r
  (bind (_returnvalue_2 _impactnormal_2) (`self.TraceFromFoot` (`self.RightFootName`) (`self.Trace Dist Below Capscule`)))
  (set `self.RightFootFoorNormal` _impactnormal_2)
  (set `self.RightFootOffset` (`KismetMathLibrary.FInterpTo` (`self.RightFootOffset`) _returnvalue_2 (`self.Delta Seconds`) (`self.Interp Speed`)))
  ;[1 1 1] Pelvis
  (set `self.PelvisFootOffset` (`KismetMathLibrary.FInterpTo` (`self.PelvisFootOffset`) (`KismetMathLibrary.FMax` (`self.LeftFootOffset`) (`self.RightFootOffset`)) (`self.Delta Seconds`) (`self.Interp Speed`)))
  (bind _rotationoffset (`self.CalculateRotationOffset` (`self.LeftFootRotation`) (`self.LeftFootFoorNormal`)))
  (set `self.LeftFootRotation` _rotationoffset)
  (bind _rotationoffset_2 (`self.CalculateRotationOffset` (`self.RightFootRotation`) (`self.RightFootFoorNormal`)))
  (set `self.RightFootRotation` _rotationoffset_2))

(fn `CalculateRotationOffset`
  (params (CurrentRotaion :type "Rotator Structure") (FloorNormal :type "Vector Structure"))
  (returns (RotationOffset :type "Rotator Structure"))
  (bind _returnvalue (`Actor.GetActorUpVector` (`self.Character`)))
  (return (`KismetMathLibrary.RInterpTo` CurrentRotaion (`KismetMathLibrary.RotatorFromAxisAndAngle` (`KismetMathLibrary.Cross_VectorVector` _returnvalue FloorNormal) (`KismetMathLibrary.DegAcos` (`KismetMathLibrary.Dot_VectorVector` _returnvalue FloorNormal))) (`self.Delta Seconds`) (`self.Interp Speed`))))

(fn `TraceFromFoot`
  (params (BoneName :type Name) (TraceDistBelowCapscule :type "Float (double-precision)"))
  (returns (ReturnValue :type "Float (double-precision)") (ImpactNormal :type "Vector Structure"))
  (locals (L_TraceDistBelowCapscule :type "Float (double-precision)") (L_BoneLocation :type "Vector Structure") (L_TraceStartLocation :type "Vector Structure") (L_TraceEndLocation :type "Vector Structure"))
  (bind (_l_bonelocation_x _l_bonelocation_y) (`KismetMathLibrary.BreakVector` (`local.L_BoneLocation`)))
  (bind (_l_bonelocation_x_2 _l_bonelocation_y_2) (`KismetMathLibrary.BreakVector` (`local.L_BoneLocation`)))
  (bind (_returnvalue_x _returnvalue_y _returnvalue_z) (`KismetMathLibrary.BreakVector` (`Actor.K2_GetActorLocation` (`self.Character`))))
  (bind (_returnvalue_x_2 _returnvalue_y_2 _returnvalue_z_2) (`KismetMathLibrary.BreakVector` (`Actor.K2_GetActorLocation` (`self.Character`))))
  (set `local.L_TraceDistBelowCapscule` TraceDistBelowCapscule)
  (set `local.L_BoneLocation` (`SceneComponent.GetSocketLocation` (`Character.Mesh` (`self.Character`)) BoneName))
  (set `local.L_TraceStartLocation` (`KismetMathLibrary.MakeVector` _l_bonelocation_x_2 _l_bonelocation_y_2 _returnvalue_z))
  (set `local.L_TraceEndLocation` (`KismetMathLibrary.MakeVector` _l_bonelocation_x _l_bonelocation_y (- _returnvalue_z_2 (+ (`CapsuleComponent.GetScaledCapsuleHalfHeight` (`Character.CapsuleComponent` (`self.Character`))) (`local.L_TraceDistBelowCapscule`)))))
  (bind (_outhit _returnvalue) (`KismetSystemLibrary.LineTraceSingle` (`local.L_TraceStartLocation`) (`local.L_TraceEndLocation`) "TraceTypeQuery2" true))
  (bind (_bblockinghit _binitialoverlap _time _distance _location _impactpoint _normal _impactnormal) (`GameplayStatics.BreakHitResult` _outhit))
  (return (`KismetMathLibrary.SelectFloat` (- (`KismetMathLibrary.VSize` (- (`local.L_TraceStartLocation`) _location)) (`CapsuleComponent.GetScaledCapsuleHalfHeight` (`Character.CapsuleComponent` (`self.Character`)))) 0.0 _returnvalue) _impactnormal))